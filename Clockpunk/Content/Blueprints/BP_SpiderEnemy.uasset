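; BP_SpiderEnemy is an enemy that walks via AI MoveTo toward the first BP_Goal actor found when play begins.
; RecieveDamage subtracts from Health, and CheckIfDead destroys the actor once Health is no longer above zero.
; Unless DebugHold is set, Tick scans every BP_Defender and turns the Cone yellow when within any defender's AttackReach, green otherwise.
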(event Custom|MoveTowardsEnemy
  (bind _outactors (Actor|GetAllActorsOfClass "/Game/Blueprints/BP_Goal.BP_Goal_C"))
  (AI|AIMoveTo self "0, 0, 0" (Utilities|Array|Get(acopy) _outactors) 5.0 false
    (:OnFail
      (Development|PrintString "Hello"))))

(event EventBeginPlay
  (CallFunction|MoveTowardsEnemy))

(event Collision|EventActorBeginOverlap
  (params (OtherActor :type Actor%20Object%20Reference)))

(event EventTick
  (params (DeltaSeconds :type Float%20%28single-precision%29))
  (if (not (Variables|Default|GetDebugHold))
    (CallFunction|DebugCheckifinRange)))

(fn ConstructionScript)

(fn CheckifDead
  (if (not (> (Variables|Default|GetHealth) 0.0))
    (Actor|DestroyActor)))

(fn RecieveDamage
  (params (Damage :type Float%20%28double-precision%29))
  (Variables|Default|SetHealth (- (Variables|Default|GetHealth) Damage))
  (CallFunction|CheckifDead))

(fn DebugCheckifinRange
  (bind _outactors (Actor|GetAllActorsOfClass "/Game/Blueprints/BP_Defender.BP_Defender_C"))
  (for _array_element _outactors
    (if (not (> (Transformation|GetDistanceTo _array_element) (Variables|/Game/Blueprints/BP_Defender.BP_Defender_C|GetAttackReach _array_element)))
      (Variables|Default|SetDebugInRange true)))
  (if (Variables|Default|GetDebugInRange)
    (Rendering|Material|SetMaterial (Variables|Default|GetCone) 0 "/Game/Materials/M_DebugMaterial_Yellow.M_DebugMaterial_Yellow")
    (else
      (Rendering|Material|SetMaterial (Variables|Default|GetCone) 0 "/Game/Materials/M_DebugMaterial_Green.M_DebugMaterial_Green")))
  (Variables|Default|SetDebugInRange false))