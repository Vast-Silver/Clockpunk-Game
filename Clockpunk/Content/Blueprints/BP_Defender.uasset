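; BP_Defender is a defender actor that periodically damages every BP_SpiderEnemy within its attack reach.
; A looping timer set on BeginPlay fires AttackEvent, which scans all spider enemies and distance-checks each one.
; Each hit calls RecieveDamage, with debug feedback that prints the distance, turns the enemy's Cone red and sets DebugHold.
; A Delay inside the loop precedes clearing DebugHold.
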(event Custom|AttackEvent
  (bind _outactors (Actor|GetAllActorsOfClass "/Game/Blueprints/BP_SpiderEnemy.BP_SpiderEnemy_C"))
  (for _array_element _outactors
    (if (< (Transformation|GetDistanceTo _array_element) (Variables|Default|GetAttackReach))
      (Development|PrintString (Utilities|String|ToString(Float) (Transformation|GetDistanceTo _array_element)))
      ;[1 1 1] Debug - Change color on in range/on hit
      (Default|RecieveDamage _array_element (Variables|Default|GetAttackDmg))
      (Variables|/Game/Blueprints/BP_SpiderEnemy.BP_SpiderEnemy_C|SetDebugHold _array_element true)
      (Rendering|Material|SetMaterial (Variables|/Game/Blueprints/BP_SpiderEnemy.BP_SpiderEnemy_C|GetCone _array_element) 0 "/Game/M_DebugMaterial_Red.M_DebugMaterial_Red")
      (Utilities|FlowControl|Delay (Variables|/Game/Blueprints/BP_SpiderEnemy.BP_SpiderEnemy_C|GetDebugTimer _array_element))
      (Variables|/Game/Blueprints/BP_SpiderEnemy.BP_SpiderEnemy_C|SetDebugHold _array_element false))))

(event EventBeginPlay
  (Utilities|Time|SetTimerbyEvent (delegate Custom|AttackEvent) (Variables|Default|GetAttackInterval) true 1.0))

(event Collision|EventActorBeginOverlap
  (params (OtherActor :type Actor%20Object%20Reference)))

(event EventTick
  (params (DeltaSeconds :type Float%20%28single-precision%29)))

(fn ConstructionScript)