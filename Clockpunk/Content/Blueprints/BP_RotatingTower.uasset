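; BP_RotatingTower is an actor that turns its Cylinder around the yaw axis by a requested angle.
; attemptRotation sets a target relative to current yaw and opens a gate that Tick feeds, adding speed-scaled rotation each frame.
; When yaw modulo 360 falls within a frame-step-scaled tolerance, it snaps to target and closes the gate.
; Angle and time histories are only seeded at BeginPlay; rotateTower is empty and the Time input is unused.
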(event Custom|attemptRotation
  (params (Time :type Float%20%28double-precision%29) (Angle :type Float%20%28double-precision%29) (RotationSpeed :type Float%20%28double-precision%29))
  (bind _cylinder (Variables|Default|GetCylinder))
  (bind _returnvalue (Transformation|GetWorldRotation _cylinder))
  (bind _returnvalue_2 (Math|Float|%(Float) (.yaw _returnvalue) 3.6e+02))
  ;[1 1 1] if tower is not rotating already, init rotation sequence
  (Variables|Default|SetisRotating true)
  (bind _output_get (Variables|Default|SetrotationTargetAngle (+ Angle (.yaw (Transformation|GetWorldRotation (Variables|Default|GetCylinder))))))
  ;[1 1 1] execute rotation within desired time
  (Utilities|FlowControl|Gate true) ; enters at Open
)

(event Custom|rotateTower)

(event EventBeginPlay
  (Utilities|Array|Add (Variables|Default|GetRotationAngleHistory) 0.0)
  (Utilities|Array|Add (Variables|Default|GetRotationTimeHistory) 0.0))

(event Collision|EventActorBeginOverlap
  (params (OtherActor :type Actor%20Object%20Reference)))

(event EventTick
  (params (DeltaSeconds :type Float%20%28single-precision%29))
  (bind _cylinder (Variables|Default|GetCylinder))
  (bind _returnvalue (Transformation|GetWorldRotation _cylinder))
  (bind _returnvalue_2 (Math|Float|%(Float) (.yaw _returnvalue) 3.6e+02))
  (Utilities|FlowControl|Sequence
    (:then_0
      ;[1 1 1] execute rotation within desired time
      (Utilities|FlowControl|Gate true :!label _label
        (:Exit
          (Transformation|AddWorldRotation _cylinder (Math|Rotator|MakeRotator 0.0 0.0 (* DeltaSeconds (stale Custom|attemptRotation RotationSpeed))) false false)
          (if (and (>= _returnvalue_2 (- (stale Custom|attemptRotation _output_get) (* (* DeltaSeconds (stale Custom|attemptRotation RotationSpeed)) (Variables|Default|GetrotationTargetTolerance)))) (<= _returnvalue_2 (+ (stale Custom|attemptRotation _output_get) (* (* DeltaSeconds (stale Custom|attemptRotation RotationSpeed)) (Variables|Default|GetrotationTargetTolerance)))))
            (Variables|Default|SetisRotating false)
            (Transformation|SetWorldRotation _cylinder (Math|Rotator|MakeRotator 0.0 0.0 (stale Custom|attemptRotation _output_get)) false false)
            (goto _label Close)))))))

(fn ConstructionScript)