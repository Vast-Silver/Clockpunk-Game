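; Desktop test pawn that drives the existing BP_VRPawn without a headset, attaching it to itself and snapping its motion controllers to hand anchors.
; Enhanced Input handles yaw-relative movement, mouse-style look and left/right grabs.
; To grab, it traces physics bodies from the camera, briefly teleports controllers to the hit or trace end (the left one always moves), calls the VR pawn's grab, then resets both.
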(event Custom|SnapControllers
  (bind _vrpawn (Variables|Default|GetVrPawn))
  (Transformation|AttachComponentToComponent (Variables|/Game/Blueprints/Player/BP_VRPawn.BP_VRPawn_C|GetMotionControllerLeft _vrpawn) (Variables|Default|GetLeftHandSnap) "None" "SnapToTarget" "SnapToTarget" "KeepRelative" true)
  (Transformation|AttachComponentToComponent (Variables|/Game/Blueprints/Player/BP_VRPawn.BP_VRPawn_C|GetMotionControllerRight _vrpawn) (Variables|Default|GetRightHandSnap) "None" "SnapToTarget" "SnapToTarget" "KeepRelative" true))

(event Input|EnhancedActionEvents|EnhancedInputActionIA_Grab_Right_NonVR
  (params (ActionValue :type Boolean) (ElapsedSeconds :type Float%20%28double-precision%29) (TriggeredSeconds :type Float%20%28double-precision%29) (InputAction :type Input%20Action%20Object%20Reference :default "/Game/Input/Actions/NonVR/IA_Grab_Right_NonVR.IA_Grab_Right_NonVR"))
  (:Started
    (CallFunction|GrabNonVR false))
  (:Completed
    (Default|StopGrabRight (Variables|Default|GetVrPawn))))

(event Input|EnhancedActionEvents|EnhancedInputActionIA_Grab_Left_NonVR
  (params (ActionValue :type Boolean) (ElapsedSeconds :type Float%20%28double-precision%29) (TriggeredSeconds :type Float%20%28double-precision%29) (InputAction :type Input%20Action%20Object%20Reference :default "/Game/Input/Actions/NonVR/IA_Grab_Left_NonVR.IA_Grab_Left_NonVR"))
  (:Started
    (CallFunction|GrabNonVR true))
  (:Completed
    (Default|StopGrabLeft (Variables|Default|GetVrPawn))))

(event Input|EnhancedActionEvents|EnhancedInputActionIA_Move_Forward_NonVR
  (params (ActionValue :type Float%20%28double-precision%29) (ElapsedSeconds :type Float%20%28double-precision%29) (TriggeredSeconds :type Float%20%28double-precision%29) (InputAction :type Input%20Action%20Object%20Reference :default "/Game/Input/Actions/NonVR/IA_Move_Forward_NonVR.IA_Move_Forward_NonVR"))
  (:Triggered
    (Pawn|Input|AddMovementInput (Math|Vector|GetForwardVector (Math|Rotator|MakeRotator 0.0 0.0 (.yaw (Pawn|GetControlRotation :!class /Script/Engine.Pawn)))) ActionValue false)))

(event Input|EnhancedActionEvents|EnhancedInputActionIA_Turn_Right_NonVR
  (params (ActionValue :type Float%20%28double-precision%29) (ElapsedSeconds :type Float%20%28double-precision%29) (TriggeredSeconds :type Float%20%28double-precision%29) (InputAction :type Input%20Action%20Object%20Reference :default "/Game/Input/Actions/NonVR/IA_Turn_Right_NonVR.IA_Turn_Right_NonVR"))
  (:Triggered
    (Pawn|Input|AddControllerYawInput ActionValue)))

(event Input|EnhancedActionEvents|EnhancedInputActionIA_LookUp_NonVR
  (params (ActionValue :type Float%20%28double-precision%29) (ElapsedSeconds :type Float%20%28double-precision%29) (TriggeredSeconds :type Float%20%28double-precision%29) (InputAction :type Input%20Action%20Object%20Reference :default "/Game/Input/Actions/NonVR/IA_LookUp_NonVR.IA_LookUp_NonVR"))
  (:Triggered
    (Pawn|Input|AddControllerPitchInput ActionValue)))

(event Input|EnhancedActionEvents|EnhancedInputActionIA_Move_Right_NonVR
  (params (ActionValue :type Float%20%28double-precision%29) (ElapsedSeconds :type Float%20%28double-precision%29) (TriggeredSeconds :type Float%20%28double-precision%29) (InputAction :type Input%20Action%20Object%20Reference :default "/Game/Input/Actions/NonVR/IA_Move_Right_NonVR.IA_Move_Right_NonVR"))
  (:Triggered
    (Pawn|Input|AddMovementInput (Math|Vector|GetRightVector (Math|Rotator|MakeRotator 0.0 0.0 (.yaw (Pawn|GetControlRotation :!class /Script/Engine.Pawn)))) ActionValue false)))

(event EventBeginPlay
  (bind _returnvalue (Actor|GetActorOfClass "/Game/Blueprints/Player/BP_VRPawn.BP_VRPawn_C"))
  (bind _output_get (Variables|Default|SetVrPawn _returnvalue))
  (Transformation|AttachActorToActor _output_get self "None" "SnapToTarget" "SnapToTarget" "SnapToTarget" true)
  (Input|AddMappingContext (PlayerController|LocalPlayerSubsystems|GetEnhancedInputLocalPlayerSubsystem (Game|GetPlayerController 0)) "/Game/Input/IMC_Default_NonVR.IMC_Default_NonVR" 0 "(bIgnoreAllPressedKeysUntilRelease=True,bForceImmediately=False)")
  (CallFunction|SnapControllers))

(fn ConstructionScript)

(fn GrabNonVR
  (params (bIsLeft :type Boolean))
  (bind _vrpawn (Variables|Default|GetVrPawn))
  (bind _camera (Variables|Default|GetCamera))
  (bind _returnvalue (Transformation|GetWorldLocation _camera))
  (bind _outhit (Collision|LineTraceForObjects _returnvalue (+ _returnvalue (* (Math|Vector|GetForwardVector _camera) 3e+02)) (Utilities|Array|MakeArray "ObjectTypeQuery4") false 0 "None"))
  (Transformation|SetWorldLocation (Variables|/Game/Blueprints/Player/BP_VRPawn.BP_VRPawn_C|GetMotionControllerLeft (Variables|Default|GetVrPawn)) (Math|Vector|SelectVector (.ImpactPoint (Collision|BreakHitResult _outhit)) (.TraceEnd (Collision|BreakHitResult _outhit)) (.bBlockingHit (Collision|BreakHitResult _outhit))) false false)
  (if bIsLeft
    (Default|StartGrabLeft _vrpawn)
    (else
      (Default|StartGrabRight _vrpawn)))
  (Transformation|SetRelativeLocation (Variables|/Game/Blueprints/Player/BP_VRPawn.BP_VRPawn_C|GetMotionControllerLeft (Variables|Default|GetVrPawn)) "0, 0, 0" false false))